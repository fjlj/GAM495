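; BP_VirusBoss2 is a virus boss that, once triggered, rotates and spawns random melee or ranged minions on a looping timer, using each spawn point once.
; Spawned minions register with the game mode, which is also notified of the boss's death shortly after its destructible mesh fractures.
; A capsule trace on Tick fires a radial impulse and light flash when objects come near, and a wrong-weapon event flashes a second light.
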(event `wrongWeapon`
  (bind _pointlight1 (`self.PointLight1`))
  (`SceneComponent.SetHiddenInGame` _pointlight1 false false)
  (`KismetSystemLibrary.Delay` 0.2)
  (`SceneComponent.SetHiddenInGame` _pointlight1 true false))

(event `/Game/BP/iface/TriggerableInterface.ActivateTriggerable`
  (`KismetSystemLibrary.Delay` (`KismetMathLibrary.RandomFloatInRange` 0.1 (`self.SpawnTimer`)))
  (`KismetSystemLibrary.K2_SetTimerDelegate` (delegate `CheckSpawnRate`) (`self.SpawnTimer`) true)
  (`AddComponent|NODE_AddRotatingMovementComponent-0`))

(event `CheckSpawnRate`
  (bind _returnvalue (`GameplayStatics.GetGameMode`))
  (bind _spawnpoints (`self.SpawnPoints`))
  (bind _returnvalue_2 (`KismetArrayLibrary.Array_Length` _spawnpoints))
  (if (> _returnvalue_2 0)
    (bind _output_get (set `self.LastPoint` (`|GetArrayItem` _spawnpoints (`KismetMathLibrary.RandomIntegerInRange` 0 (- _returnvalue_2 1)))))
    (bind _returnvalue_3 (`|SpawnActorFromClass` (castclass `/Game/BP/AI/BaseAI/BP_BaseNPC` (select `int` (`KismetMathLibrary.RandomIntegerInRange` 0 1) :`0` "/Game/BP/AI/BaseAI/BP_RangedEnemy.BP_RangedEnemy_C" :`1` "/Game/BP/AI/BaseAI/BP_MeleeEnemy.BP_MeleeEnemy_C" :!type "Actor Class Reference") :!pure true) (`self.GetTransform` _output_get) "Undefined" "OverrideRootScale" null null true null))
    (message `/Game/BP/iface/AIInterface.RegisterAI` _returnvalue _returnvalue_3)
    (message `/Game/BP/iface/AIInterface.RegisterBossMinion` _returnvalue _returnvalue_3)
    (`KismetArrayLibrary.Array_RemoveItem` (`self.SpawnPoints`) (`self.LastPoint`))))

(event `self.Virus2_DM.OnComponentFracture`
  (params (HitPoint :type "Vector Structure (by ref)") (HitDirection :type "Vector Structure (by ref)"))
  (`KismetSystemLibrary.Delay` 2.25)
  (message `/Game/BP/iface/AIInterface.NotifyBossDeath` (`GameplayStatics.GetGameMode`) (`self.BossIndex`))
  (`self.K2_DestroyActor` (`ActorComponent.GetOwner` (`self.Virus2_DM`))))

(event `self.ReceiveTick`
  (params (DeltaSeconds :type "Float (single-precision)"))
  (bind (_returnvalue_x _returnvalue_y _returnvalue_z) (`KismetMathLibrary.BreakVector` (`self.K2_GetActorLocation`)))
  (bind (_outhit _returnvalue) (`KismetSystemLibrary.CapsuleTraceSingleForObjects` (`KismetMathLibrary.MakeVector` _returnvalue_x (- _returnvalue_y 50.0) _returnvalue_z) (`KismetMathLibrary.MakeVector` 0.0 (+ _returnvalue_y 50.0)) 250.0 0.0 (`|MakeArray` "ObjectTypeQuery7" "ObjectTypeQuery8" "ObjectTypeQuery10" "ObjectTypeQuery5" "ObjectTypeQuery4" :!type "EObjectTypeQuery Enum")))
  (if _returnvalue
    (`RadialForceComponent.FireImpulse` (`self.RadialForce`))
    (`SceneComponent.SetHiddenInGame` (`self.PointLight`) false false)
    (`KismetSystemLibrary.Delay` 0.2)
    (`SceneComponent.SetHiddenInGame` (`self.PointLight`) true false)))

(fn `UserConstructionScript`
  (`parent.UserConstructionScript`))