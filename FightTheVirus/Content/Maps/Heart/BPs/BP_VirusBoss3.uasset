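; BP_VirusBoss3 is the third virus boss in the Heart map, a destructible enemy that starts rotating and attacking when triggered.
; A looping timer fires a shot toward the player and spawns random melee or ranged minions, lowering SpawnTimer without re-arming the timer.
; Tick capsule-traces for nearby objects to fire a radial impulse with a light flash; wrongWeapon flashes another light.
; Fracturing notifies the game mode of boss death and destroys it after a delay.
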(event `wrongWeapon`
  (bind _pointlight1 (`self.PointLight1`))
  (`SceneComponent.SetHiddenInGame` _pointlight1 false false)
  (`KismetSystemLibrary.Delay` 0.2)
  (`SceneComponent.SetHiddenInGame` _pointlight1 true false))

(event `/Game/BP/iface/TriggerableInterface.ActivateTriggerable`
  (`KismetSystemLibrary.Delay` (`KismetMathLibrary.RandomFloatInRange` 0.01 (`KismetMathLibrary.FClamp` (`self.SpawnTimer`) 0.0 1.15)))
  (`KismetSystemLibrary.K2_SetTimerDelegate` (delegate `CheckSpawnRate`) (`self.SpawnTimer`) true)
  (`AddComponent|NODE_AddRotatingMovementComponent-0`))

(event `CheckSpawnRate`
  (bind _returnvalue (`GameplayStatics.GetGameMode`))
  (bind _spawnpoints (`self.SpawnPoints`))
  (bind _returnvalue_2 (`KismetArrayLibrary.Array_Length` _spawnpoints))
  (if (> _returnvalue_2 0)
    (bind _output_get (set `self.LastPoint` (`|GetArrayItem` _spawnpoints (`KismetMathLibrary.RandomIntegerInRange` 0 (- _returnvalue_2 1)))))
    (`|SpawnActorFromClass` "/Game/BP/AI/AIAttacks/BP_EnemyRangedFire_2.BP_EnemyRangedFire_2_C" (`KismetMathLibrary.MakeTransform` (+ (+ (`self.K2_GetActorLocation`) (* (`self.GetActorForwardVector`) 100.0)) (0.0 0.0 40.0)) (`KismetMathLibrary.Conv_VectorToRotator` (`KismetMathLibrary.Normal` (- (`self.K2_GetActorLocation` (`GameplayStatics.GetPlayerCharacter` 0)) (`self.K2_GetActorLocation`))))) "Undefined" "OverrideRootScale" self 10.0 null null)
    (`GameplayStatics.SpawnSoundAtLocation` "/Game/SFX/Enemy_Shot.Enemy_Shot" (`self.K2_GetActorLocation` self) (struct) 0.075 1.0 0.0 null "/Game/SFX/FXConcurrency.FXConcurrency")
    (bind _returnvalue_3 (`|SpawnActorFromClass` (castclass `/Game/BP/AI/BaseAI/BP_BaseNPC` (select `int` (`KismetMathLibrary.RandomIntegerInRange` 0 1) :`0` "/Game/BP/AI/BaseAI/BP_RangedEnemy.BP_RangedEnemy_C" :`1` "/Game/BP/AI/BaseAI/BP_MeleeEnemy.BP_MeleeEnemy_C" :!type "Actor Class Reference") :!pure true) (`self.GetTransform` _output_get) "Undefined" "OverrideRootScale" null null true null))
    (if (`KismetSystemLibrary.IsValid` _returnvalue_3)
      (message `/Game/BP/iface/AIInterface.RegisterAI` _returnvalue _returnvalue_3)
      (message `/Game/BP/iface/AIInterface.RegisterBossMinion` _returnvalue null)
      (set `self.SpawnTimer` (- (`self.SpawnTimer`) 0.105)))))

(event `self.Virus3_DM.OnComponentFracture`
  (params (HitPoint :type "Vector Structure (by ref)") (HitDirection :type "Vector Structure (by ref)"))
  (`KismetSystemLibrary.Delay` 2.98)
  (message `/Game/BP/iface/AIInterface.NotifyBossDeath` (`GameplayStatics.GetGameMode`) (`self.BossIndex`))
  (`self.K2_DestroyActor` (`ActorComponent.GetOwner` (`self.Virus3_DM`))))

(event `self.ReceiveTick`
  (params (DeltaSeconds :type "Float (single-precision)"))
  (bind (_returnvalue_x _returnvalue_y _returnvalue_z) (`KismetMathLibrary.BreakVector` (`self.K2_GetActorLocation`)))
  (bind (_outhit _returnvalue) (`KismetSystemLibrary.CapsuleTraceSingleForObjects` (`KismetMathLibrary.MakeVector` _returnvalue_x (+ _returnvalue_y 50.0) _returnvalue_z) (`KismetMathLibrary.MakeVector` _returnvalue_x (- _returnvalue_y 50.0) _returnvalue_z) 500.0 0.0 (`|MakeArray` "ObjectTypeQuery7" "ObjectTypeQuery8" "ObjectTypeQuery10" "ObjectTypeQuery5" "ObjectTypeQuery4" :!type "EObjectTypeQuery Enum")))
  (if _returnvalue
    (`RadialForceComponent.FireImpulse` (`self.RadialForce`))
    (`SceneComponent.SetHiddenInGame` (`self.PointLight`) false false)
    (`KismetSystemLibrary.Delay` 0.2)
    (`SceneComponent.SetHiddenInGame` (`self.PointLight`) true false)))

(fn `UserConstructionScript`
  (`parent.UserConstructionScript`))