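; BP_AISpawner is a placeable spawn point that creates one AI NPC when the player character comes within its activation distance.
; After a random startup delay, a looping timer checks distance to player 0.
; When in range, it spawns the enemy or friendly cell class selected by AIType, passes on LinkedTeleporter, then clears the timer and destroys itself.
; The construction script shows the selected type on a text component.
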(event `self.ReceiveBeginPlay`
  (`KismetSystemLibrary.Delay` (`KismetMathLibrary.RandomFloatInRange` 0.1 (`self.CheckTimerTick`)))
  (bind _returnvalue (`KismetSystemLibrary.K2_SetTimerDelegate` (delegate `DistanceCheck`) (`self.CheckTimerTick`) true))
  (set `self.CheckPlayerDistanceTimer` _returnvalue))

(event `DistanceCheck`
  (bind (_returnvalue_location _returnvalue_rotation) (`KismetMathLibrary.BreakTransform` (`self.GetTransform`)))
  (if (> (`self.ActivationDistance`) (`KismetMathLibrary.VSize` (- (`self.K2_GetActorLocation`) (`self.K2_GetActorLocation` (`GameplayStatics.GetPlayerCharacter` 0)))))
    (`|SpawnActorFromClass` (castclass `/Game/BP/AI/BaseAI/BP_BaseNPC` (select `/Game/BP/AI/E_AI_Type` (`self.AI Type`) :`NewEnumerator0` "/Game/BP/AI/BaseAI/BP_RangedEnemy.BP_RangedEnemy_C" :`NewEnumerator1` "/Game/BP/AI/BaseAI/BP_MeleeEnemy.BP_MeleeEnemy_C" :`NewEnumerator2` "/Game/BP/AI/BaseAI/BP_RangedWhiteCell.BP_RangedWhiteCell_C" :`NewEnumerator3` "/Game/BP/AI/BaseAI/BP_MeleeRedCell.BP_MeleeRedCell_C" :!type "Actor Class Reference") :!pure true) (`KismetMathLibrary.MakeTransform` _returnvalue_location _returnvalue_rotation) "Undefined" "OverrideRootScale" null (`self.LinkedTeleporter`) false null)
    (`KismetSystemLibrary.K2_ClearAndInvalidateTimerHandle` (`self.CheckPlayerDistanceTimer`))
    (`self.K2_DestroyActor`)))

(fn `UserConstructionScript`
  (`TextRenderComponent.K2_SetText` (`self.Type Text`) (`KismetTextLibrary.Conv_StringToText` (`|GetEnumeratorNameAsString` (`self.AI Type`)))))