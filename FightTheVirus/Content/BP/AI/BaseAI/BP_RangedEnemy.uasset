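; BP_RangedEnemy is an AI enemy whose attack fires a ranged projectile at its target.
; On AIAttack with a valid target, it spawns a BP_EnemyRangedFire_2 actor offset forward and upward from itself, rotated along the direction from its location to the target.
; It owns the spawned actor and plays a quiet shot sound at its location under a concurrency setting.
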(event `/Game/BP/iface/AIInterface.AIAttack`
  (params (Target :type "Actor Object Reference"))
  (`/Engine/EditorBlueprintResources/StandardMacros.IsValid` Target
    (:`Is Valid`
      (`|SpawnActorFromClass` "/Game/BP/AI/AIAttacks/BP_EnemyRangedFire_2.BP_EnemyRangedFire_2_C" (`KismetMathLibrary.MakeTransform` (+ (+ (`self.K2_GetActorLocation`) (* (`self.GetActorForwardVector`) (`self.Spawn Forward Offset`))) (`KismetMathLibrary.MakeVector` 0.0 0.0 (`self.Spawn Z Offset`))) (`KismetMathLibrary.Conv_VectorToRotator` (`KismetMathLibrary.Normal` (- (`self.K2_GetActorLocation` Target) (`self.K2_GetActorLocation`))))) "Undefined" "OverrideRootScale" self 10.0 null null)
      (`GameplayStatics.SpawnSoundAtLocation` "/Game/SFX/Enemy_Shot.Enemy_Shot" (`self.K2_GetActorLocation` self) (struct) 0.075 1.0 0.0 null "/Game/SFX/FXConcurrency.FXConcurrency"))))

(fn `UserConstructionScript`
  (`parent.UserConstructionScript`))