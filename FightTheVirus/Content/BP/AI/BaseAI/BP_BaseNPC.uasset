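; Base NPC actor that runs a behavior tree, registers with the game mode and manages health and death.
; Damage sets a temporary blackboard aggro target, except player hits on Coop-tagged NPCs, which recalculate health through a clamped heal formula.
; Death unregisters it, notifies any linked teleporter and spawns a ranged enemy for Coop NPCs.
; Tick drives optional mesh hovering and turns the visible health bar toward the player; AIAttack only prints.
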(event `self.ReceiveAnyDamage`
  (params (Damage :type "Float (single-precision)") (DamageType :type "DamageType Object Reference") (InstigatedBy :type "Controller Object Reference") (DamageCauser :type "Actor Object Reference"))
  (bind _returnvalue (`AIBlueprintHelperLibrary.GetBlackboard` self))
  ;[1 1 1] Damage
  (if (and (== (`GameplayStatics.GetPlayerCharacter` 0) DamageCauser) (`self.ActorHasTag` "Coop"))
    (set `self.CurrentHealth` (`KismetMathLibrary.FClamp` (+ (* (`self.CurrentHealth`) (`self.Heal Damage %`)) Damage) 0.0 (`self.MaxHealth`)))
    (`self.HP Updated`)
    (else
      (bind _output_get (set `self.CurrentHealth` (- (`self.CurrentHealth`) Damage)))
      (`self.HP Updated`)
      (if (<= _output_get 0.0)
        (`self.Die`)
        (else
          (`/Engine/EditorBlueprintResources/StandardMacros.IsValid` DamageCauser
            (:`Is Valid`
              (`BlackboardComponent.SetValueAsBool` _returnvalue "DamagedRecently" true)
              (`BlackboardComponent.SetValueAsObject` _returnvalue "Target" DamageCauser)
              (`KismetSystemLibrary.RetriggerableDelay` (`self.AggroTimer`))
              (`BlackboardComponent.SetValueAsBool` _returnvalue "DamagedRecently" false))))))))

(event `self.ReceiveTick`
  (params (DeltaSeconds :type "Float (single-precision)"))
  (bind _staticmesh (`self.StaticMesh`))
  (bind (_relativelocation_x _relativelocation_y) (`KismetMathLibrary.BreakVector` (`SceneComponent.RelativeLocation` _staticmesh)))
  ;[1 1 1] Tick Float
  (`|ExecutionSequence`
    (:`then_0`
      (if (`self.TickFloat`)
        (if (`self.GoingUp`)
          (bind _output_get (set `self.CurrentHoverHeight` (+ (* (`self.HoverSpeed`) DeltaSeconds) (`self.CurrentHoverHeight`))))
          (if (> _output_get (`self.HoverHeight`))
            (set `self.CurrentHoverHeight` (`self.HoverHeight`))
            (set `self.GoingUp` false))
          (else
            (bind _output_get_2 (set `self.CurrentHoverHeight` (- (`self.CurrentHoverHeight`) (* (`self.HoverSpeed`) DeltaSeconds))))
            (if (< _output_get_2 (* -1 (`self.HoverHeight`)))
              (set `self.CurrentHoverHeight` (* -1 (`self.HoverHeight`)))
              (set `self.GoingUp` true))))
        (`SceneComponent.K2_SetRelativeLocation` _staticmesh (`KismetMathLibrary.MakeVector` _relativelocation_x _relativelocation_y (`self.CurrentHoverHeight`)) false true)))
    (:`then_1`
      ;[1 1 1] TickBarRotation
      (if (`self.HPBarVisible`)
        (`self.RotateBarToPlayer`)))))

(event `/Game/BP/iface/AIInterface.AIAttack`
  (params (Target :type "Actor Object Reference"))
  ;[1 1 1] Attack
  (`KismetSystemLibrary.PrintString` (`KismetStringLibrary.Concat_StrStr` "Attack: " (`KismetSystemLibrary.GetDisplayName` Target))))

(event `Die`
  (bind _returnvalue (`GameplayStatics.GetGameMode`))
  (bind _linkedteleporter (`self.LinkedTeleporter`))
  ;[1 1 1] Death
  (message `/Game/BP/iface/AIInterface.UnregisterAI` _returnvalue self)
  (if (`self.BossSpawn?`)
    (message `/Game/BP/iface/AIInterface.UnregisterBossMinion` _returnvalue self))
  (`/Engine/EditorBlueprintResources/StandardMacros.IsValid` _linkedteleporter
    (:`Is Valid`
      (`/Game/BP/GameplayItems/MovementItems/BP_Teleporter.ActorDied` _linkedteleporter self))
    (:`Is Not Valid`
      _))
  (if (`self.ActorHasTag` "Coop")
    (`|SpawnActorFromClass` "/Game/BP/AI/BaseAI/BP_RangedEnemy.BP_RangedEnemy_C" (`self.GetTransform`) "AlwaysSpawn" "OverrideRootScale" null null false null))
  (`self.K2_DestroyActor`))

(event `self.ReceiveBeginPlay`
  (bind _linkedteleporter (`self.LinkedTeleporter`))
  ;[1 1 1] Init
  (message `/Game/BP/iface/AIInterface.RegisterAI` (`GameplayStatics.GetGameMode`) self)
  (`AIController.RunBehaviorTree` (`AIBlueprintHelperLibrary.GetAIController` self) (`self.BT`))
  (set `self.CurrentHealth` (`self.MaxHealth`))
  (`/Engine/EditorBlueprintResources/StandardMacros.IsValid` _linkedteleporter
    (:`Is Valid`
      (`/Game/BP/GameplayItems/MovementItems/BP_Teleporter.Add AI To clear` _linkedteleporter self))
    (:`Is Not Valid`
      _))
  (bind _asui_npchp (cast `/Game/BP/AI/UI_NPCHP` (`WidgetComponent.GetUserWidgetObject` (`self.Widget`))))
  (bind _output_get (set `self.HP Bar` _asui_npchp))
  (set `/Game/BP/AI/UI_NPCHP.Owner` self _output_get))

(event `/Game/BP/iface/AIInterface.ShowHealthBar`
  ;[1 1 1] HP Bar Handling
  (set `self.HPBarVisible` true)
  (`SceneComponent.SetHiddenInGame` (`self.Widget`) false false)
  (`self.RotateBarToPlayer`))

(event `/Game/BP/iface/AIInterface.HideHealthBar`
  ;[1 1 1] HP Bar Handling
  (`KismetSystemLibrary.RetriggerableDelay` 2.0)
  (set `self.HPBarVisible` false)
  (`SceneComponent.SetHiddenInGame` (`self.Widget`) true false))

(event `RotateBarToPlayer`
  (bind (_returnvalue_roll _returnvalue_pitch _returnvalue_yaw) (`KismetMathLibrary.BreakRotator` (`KismetMathLibrary.FindLookAtRotation` (`self.K2_GetActorLocation`) (`self.K2_GetActorLocation` (`GameplayStatics.GetPlayerCharacter` 0)))))
  ;[1 1 1] HP Bar Handling
  (`SceneComponent.K2_SetWorldRotation` (`self.Widget`) (`KismetMathLibrary.MakeRotator` 0.0 0.0 _returnvalue_yaw) false false))

(event `Update HP Bar`
  ;[1 1 1] HP Bar Handling
  (`/Game/BP/AI/UI_NPCHP.SetPercent` (`self.HP Bar`) (/ (`self.CurrentHealth`) (`self.MaxHealth`))))

(fn `GetAIActors`
  (returns (NewParam :type "Array of Actor Object Reference"))
  (return))

(fn `GetHP`
  (returns (Health :type "Float (double-precision)") (MaxHealth :type "Float (double-precision)"))
  (return (`self.CurrentHealth`) (`self.MaxHealth`)))

(fn `UserConstructionScript`)