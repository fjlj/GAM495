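; BP_MeleeRedCell is an AI character Blueprint that implements a melee attack.
; On AIAttack with a valid target, it spawns a BP_CoopMelee actor at forward and vertical offsets, facing the AI's rotation, and plays the melee sound there.
; An unconnected branch that spawns a BP_CoopRangedFire_2 projectile never runs.
; BeginPlay, overlap and Tick are inactive stubs, and the construction script only calls its parent.
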(event `/Game/BP/iface/AIInterface.AIAttack`
  (params (Target :type "Actor Object Reference"))
  (bind _returnvalue (+ (+ (`self.K2_GetActorLocation`) (* (`self.GetActorForwardVector`) (`self.Attack Forward Spawn Offset`))) (`KismetMathLibrary.MakeVector` 0.0 0.0 (`self.Attack Z Spawn offset`))))
  (`/Engine/EditorBlueprintResources/StandardMacros.IsValid` Target
    (:`Is Valid`
      (`|SpawnActorFromClass` "/Game/BP/AI/AIAttacks/BP_CoopMelee.BP_CoopMelee_C" (`KismetMathLibrary.MakeTransform` _returnvalue (`self.K2_GetActorRotation`)) "Undefined" "OverrideRootScale" null 25.0 null)
      (`GameplayStatics.SpawnSoundAtLocation` "/Game/SFX/Melee_Attack.Melee_Attack" _returnvalue (struct) 0.25 1.0 0.0 null "/Game/SFX/FXConcurrency.FXConcurrency"))))

(fn `UserConstructionScript`
  (`parent.UserConstructionScript`))