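; BP_CoopMelee is a short-lived melee hit actor that damages an actor tagged Enemy.
; Its sphere starts at zero radius, expands to Radius on BeginPlay, and the actor destroys itself after a brief delay.
; The first qualifying overlap passes a DoOnce and applies Damage, with a random chance of bonus crit damage, so each instance hits only one enemy.
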(event `self.ReceiveBeginPlay`
  (`SphereComponent.SetSphereRadius` (`self.Sphere`) (`self.Radius`) true)
  (`KismetSystemLibrary.Delay` 0.2)
  (`self.K2_DestroyActor`))

(event `self.Sphere.OnComponentBeginOverlap`
  (params (OverlappedComponent :type "PrimitiveComponent Object Reference") (OtherActor :type "Actor Object Reference") (OtherComp :type "PrimitiveComponent Object Reference") (OtherBodyIndex :type Integer) (bFromSweep :type Boolean) (SweepResult :type "HitResult Structure (by ref)"))
  (if (`self.ActorHasTag` OtherActor "Enemy")
    (`/Engine/EditorBlueprintResources/StandardMacros.DoOnce` false
      (:`Completed`
        (if (>= (`KismetMathLibrary.RandomFloatInRange` 0.0 1.0) 0.8)
          (bind _output_get (set `self.Damage_crit` (`KismetMathLibrary.RandomFloatInRange` 2.0 10.0))))
        (`GameplayStatics.ApplyDamage` OtherActor (+ _output_get (`self.Damage`)))
        (set `self.Damage_crit` 0.0)
        (`KismetSystemLibrary.PrintString` "Attacked")))))

(fn `UserConstructionScript`
  (`SphereComponent.SetSphereRadius` (`self.Sphere`) 0.0 true))