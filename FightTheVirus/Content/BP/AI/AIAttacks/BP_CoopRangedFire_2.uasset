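; BP_CoopRangedFire_2 is a ranged attack projectile that damages actors tagged "Enemy" on behalf of its owner.
; A looping timer replaces per-frame Tick, sphere tracing from the previous position to the current one to catch hits between updates while ignoring the owner.
; Enemy hits apply base damage plus an occasional random crit bonus.
; Any valid hit, enemy or not, stops the timer and destroys the projectile.
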(event `self.ReceiveBeginPlay`
  (set `self.PreviousLocation` (`self.K2_GetActorLocation`))
  (bind _returnvalue (`KismetSystemLibrary.K2_SetTimerDelegate` (delegate `Tick`) (`self.TickFrequency`) true))
  (set `self.TickTimer` _returnvalue)
  (`self.Tick`))

(event `Tick`
  (bind (_outhit _returnvalue) (`KismetSystemLibrary.SphereTraceSingleForObjects` (`self.PreviousLocation`) (`self.K2_GetActorLocation`) (`self.TraceRadius`) (`|MakeArray` "ObjectTypeQuery1" "ObjectTypeQuery2" "ObjectTypeQuery3" :!type "EObjectTypeQuery Enum") false (`|MakeArray` (`self.OwnerActor`)) (select `bool` (`self.Debug?`) :`true` "ForDuration" :!type "EDrawDebugTrace Enum")))
  (if _returnvalue
    (bind (_bblockinghit _binitialoverlap _time _distance _location _impactpoint _normal _impactnormal _physmat _hitactor) (`GameplayStatics.BreakHitResult` _outhit))
    (`/Engine/EditorBlueprintResources/StandardMacros.IsValid` _hitactor
      (:`Is Valid`
        (if (`self.ActorHasTag` _hitactor "Enemy")
          (if (>= (`KismetMathLibrary.RandomFloatInRange` 0.0 1.0) 0.8)
            (bind _output_get (set `self.Damage_crit` (`KismetMathLibrary.RandomFloatInRange` 1.0 7.0))))
          (`GameplayStatics.ApplyDamage` _hitactor (+ _output_get (`self.Damage`)) null (`self.OwnerActor`))
          (set `self.Damage_crit` 0.0))
        (`KismetSystemLibrary.K2_ClearAndInvalidateTimerHandle` (`self.TickTimer`))
        (`self.K2_DestroyActor`)))
    (else
      (set `self.PreviousLocation` (`self.K2_GetActorLocation`)))))

(fn `UserConstructionScript`)