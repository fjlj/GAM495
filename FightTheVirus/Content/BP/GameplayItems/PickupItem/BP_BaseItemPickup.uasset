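; Base pickup item actor that the player collects by touching it, delivering an item type and value.
; On capsule overlap with a Player-tagged actor, it fires PickupItemMessage on that actor once, then destroys itself.
; An optionally enabled Tick spins the pickup around yaw at a configurable speed.
; The construction script applies a dynamic M_Emissive material tinted by a configurable color.
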(event `self.ReceiveBeginPlay`
  (`self.SetActorTickEnabled` (`self.EnableTick?`))
  (set `self.TickRate` (`self.TickRate`)))

(event `self.ReceiveTick`
  (params (DeltaSeconds :type "Float (single-precision)"))
  (`SceneComponent.K2_AddLocalRotation` (`self.PickupRotation`) (`KismetMathLibrary.MakeRotator` 0.0 0.0 (`self.TickRotationSpeed`)) false false))

(event `self.Capsule.OnComponentBeginOverlap`
  (params (OverlappedComponent :type "PrimitiveComponent Object Reference") (OtherActor :type "Actor Object Reference") (OtherComp :type "PrimitiveComponent Object Reference") (OtherBodyIndex :type Integer) (bFromSweep :type Boolean) (SweepResult :type "HitResult Structure (by ref)"))
  (if (`self.ActorHasTag` OtherActor "Player")
    (`/Engine/EditorBlueprintResources/StandardMacros.DoOnce` false
      (:`Completed`
        (message `/Game/BP/iface/InteractableInterface.PickupItem` OtherActor (`self.ItemType`) (`self.AddedValue`))
        (`self.K2_DestroyActor`)))))

(fn `UserConstructionScript`
  (bind _returnvalue (`KismetMaterialLibrary.CreateDynamicMaterialInstance` "/Game/Materials/M_Emissive.M_Emissive"))
  (bind _output_get (set `self.DynamicMaterial` _returnvalue))
  (`PrimitiveComponent.SetMaterial` (`self.StaticMesh`) 0 _output_get)
  (`MaterialInstanceDynamic.SetVectorParameterValue` (`self.DynamicMaterial`) "Color" (`self.MaterialColor`)))