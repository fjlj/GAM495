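; Standard player projectile shaped like a two-part pill, given random colours on each half and a random spin at spawn.
; A looping timer, rather than actor tick, sphere-traces from the previous location to the current one, ignoring the player, to catch hits between updates.
; A hit applies base damage, plus random bonus "crit" damage on 92% of rolls, credited to the player, then destroys the shot.
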(event `self.ReceiveBeginPlay`
  (bind _returnvalue (`KismetMathLibrary.MakeColor` (`KismetMathLibrary.RandomFloatInRange` 0.0 1.0) (`KismetMathLibrary.RandomFloatInRange` 0.0 1.0) (`KismetMathLibrary.RandomFloatInRange` 0.0 1.0)))
  (`MaterialInstanceDynamic.SetVectorParameterValue` (`self.CapBotDM`) "PillColor" _returnvalue)
  (`MaterialInstanceDynamic.SetVectorParameterValue` (`self.CapTopDM`) "PillColor" _returnvalue)
  (set `RotatingMovementComponent.RotationRate` (`KismetMathLibrary.RandomRotator` true) (`self.RotatingMovement`))
  (set `self.PreviousLocation` (`self.K2_GetActorLocation`))
  (bind _returnvalue_2 (`KismetSystemLibrary.K2_SetTimerDelegate` (delegate `Tick`) (`self.TickFrequency`) true))
  (set `self.TickTimer` _returnvalue_2)
  (`self.Tick`))

(event `Tick`
  (bind (_outhit _returnvalue) (`KismetSystemLibrary.SphereTraceSingleForObjects` (`self.PreviousLocation`) (`self.K2_GetActorLocation`) (`self.TraceRadius`) (`|MakeArray` "ObjectTypeQuery1" "ObjectTypeQuery2" "ObjectTypeQuery3" "ObjectTypeQuery6" :!type "EObjectTypeQuery Enum") false (`|MakeArray` (`GameplayStatics.GetPlayerCharacter` 0) :!type "Actor Object Reference") (select `bool` (`self.Debug?`) :`true` "ForDuration" :!type "EDrawDebugTrace Enum")))
  (if _returnvalue
    (if (<= (`KismetMathLibrary.RandomFloatInRange` 0.0 1.0) 0.92)
      (set `self.crit_damage` (`KismetMathLibrary.RandomFloatInRange` 15.0 30.0)))
    (`GameplayStatics.ApplyDamage` (`.HitActor` (`GameplayStatics.BreakHitResult` _outhit)) (+ (`self.Damage`) (`self.crit_damage`)) (`GameplayStatics.GetPlayerController` 0) (`GameplayStatics.GetPlayerCharacter` 0))
    (set `self.crit_damage` 0.0)
    (`KismetSystemLibrary.K2_ClearAndInvalidateTimerHandle` (`self.TickTimer`))
    (`self.K2_DestroyActor`)
    (else
      (set `self.PreviousLocation` (`self.K2_GetActorLocation`)))))

(fn `UserConstructionScript`
  (bind _returnvalue (`PrimitiveComponent.CreateDynamicMaterialInstance` (`self.CapsuleBottom`) 0 null "None"))
  (set `self.CapBotDM` _returnvalue)
  (bind _returnvalue_2 (`PrimitiveComponent.CreateDynamicMaterialInstance` (`self.CapsuleTop`) 0 null "None"))
  (set `self.CapTopDM` _returnvalue_2))