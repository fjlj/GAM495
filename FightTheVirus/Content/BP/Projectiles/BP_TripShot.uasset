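; BP_TripShot is a spawner actor that turns one shot into a three-projectile horizontal spread.
; On BeginPlay it spawns three actors at its own location: one along its rotation and two yawed by plus and minus ZSpread.
; Each receives DamagePerProjectile as its Damage and spawns regardless of collision, then the spawner immediately destroys itself.
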(event `self.ReceiveBeginPlay`
  (bind (_returnvalue_location _returnvalue_rotation) (`KismetMathLibrary.BreakTransform` (`self.GetTransform`)))
  (bind (_returnvalue_location_2 _returnvalue_rotation_2) (`KismetMathLibrary.BreakTransform` (`self.GetTransform`)))
  (bind (_returnvalue_location_3 _returnvalue_rotation_3) (`KismetMathLibrary.BreakTransform` (`self.GetTransform`)))
  (`|SpawnActorFromClass` "/Game/BP/Projectiles/BP_StandardShot.BP_StandardShot_C" (`KismetMathLibrary.MakeTransform` _returnvalue_location_2 _returnvalue_rotation_2) "AlwaysSpawn" "OverrideRootScale" null (`self.DamagePerProjectile`) null)
  (`|SpawnActorFromClass` "/Game/BP/Projectiles/BP_StandardShot.BP_StandardShot_C" (`KismetMathLibrary.MakeTransform` _returnvalue_location_3 (`KismetMathLibrary.ComposeRotators` _returnvalue_rotation_3 (`KismetMathLibrary.MakeRotator` 0.0 0.0 (`self.ZSpread`)))) "AlwaysSpawn" "OverrideRootScale" null (`self.DamagePerProjectile`) null)
  (`|SpawnActorFromClass` "/Game/BP/Projectiles/BP_StandardShot.BP_StandardShot_C" (`KismetMathLibrary.MakeTransform` _returnvalue_location (`KismetMathLibrary.ComposeRotators` _returnvalue_rotation (`KismetMathLibrary.MakeRotator` 0.0 0.0 (* (`self.ZSpread`) -1.0)))) "AlwaysSpawn" "OverrideRootScale" null (`self.DamagePerProjectile`) null)
  (`self.K2_DestroyActor`))

(fn `UserConstructionScript`)