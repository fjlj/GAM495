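; BP_Explosion is a short-lived explosion actor that deals area damage to actors not tagged Player.
; Its sphere starts at zero radius in construction, then expands to Radius on BeginPlay with overlap updates, and the actor destroys itself shortly after.
; Sphere begin-overlap events apply Damage, credited to the first player's controller and character.
; An older loop over overlapping actors is left disconnected.
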(event `self.ReceiveBeginPlay`
  (`SphereComponent.SetSphereRadius` (`self.Sphere`) (`self.Radius`) true)
  (`KismetSystemLibrary.Delay` 0.2)
  (`self.K2_DestroyActor`))

(event `self.Sphere.OnComponentBeginOverlap`
  (params (OverlappedComponent :type "PrimitiveComponent Object Reference") (OtherActor :type "Actor Object Reference") (OtherComp :type "PrimitiveComponent Object Reference") (OtherBodyIndex :type Integer) (bFromSweep :type Boolean) (SweepResult :type "HitResult Structure (by ref)"))
  (if (not (`self.ActorHasTag` OtherActor "Player"))
    (`GameplayStatics.ApplyDamage` OtherActor (`self.Damage`) (`GameplayStatics.GetPlayerController` 0) (`GameplayStatics.GetPlayerCharacter` 0))))

(fn `UserConstructionScript`
  (`SphereComponent.SetSphereRadius` (`self.Sphere`) 0.0 true))