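; Short-lived player laser shot: a hitscan projectile drawn as a particle beam.
; On spawn it sphere-traces forward, damages the hit actor and ends the beam at the impact or trace end, while Tick keeps the beam source on the player's gun.
; Construction sizes a cylinder to the trace distance and sets the lifespan.
; Overlaps of Cylinder1 with boss-tagged components call WrongWeapon on the matching virus boss, found by class name.
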(event `self.ReceiveBeginPlay`
  (bind _returnvalue (`self.K2_GetActorLocation`))
  (bind _asfirst_person_character (cast `/Game/FirstPersonBP/Blueprints/FirstPersonCharacter` (`GameplayStatics.GetPlayerCharacter` 0)))
  (bind _output_get (set `self.Player` _asfirst_person_character))
  (bind (_valid_ _location) (message `/Game/BP/iface/InteractableInterface.GetGunLocation` _output_get))
  (if _valid_
    (`ParticleSystemComponent.SetBeamSourcePoint` (`self.ParticleSystem`) 0 _location 0)
    (bind (_outhit _returnvalue_2) (`KismetSystemLibrary.SphereTraceSingleForObjects` _returnvalue (+ _returnvalue (* (`self.GetActorForwardVector`) (`self.Trace Distance`))) (`self.SphereRadius`) (`|MakeArray` "ObjectTypeQuery1" "ObjectTypeQuery2" "ObjectTypeQuery3" :!type "EObjectTypeQuery Enum") false (`|MakeArray` (`GameplayStatics.GetPlayerCharacter` 0) :!type "Actor Object Reference") (select `bool` (`self.Debug?`) :`true` "ForDuration" :!type "EDrawDebugTrace Enum")))
    (if _returnvalue_2
      (bind (_bblockinghit _binitialoverlap _time _distance _location_2 _impactpoint _normal _impactnormal _physmat _hitactor _hitcomponent _hitbonename _hititem _faceindex _tracestart _traceend) (`GameplayStatics.BreakHitResult` _outhit))
      (`ParticleSystemComponent.SetBeamEndPoint` (`self.ParticleSystem`) 0 _impactpoint)
      (`GameplayStatics.ApplyDamage` _hitactor (`self.Damage`) (`GameplayStatics.GetPlayerController` 0) (`GameplayStatics.GetPlayerCharacter` 0))
      (if (`self.Debug?`)
        _)
      (else
        (`ParticleSystemComponent.SetBeamEndPoint` (`self.ParticleSystem`) 0 _traceend)))))

(event `self.ReceiveTick`
  (params (DeltaSeconds :type "Float (single-precision)"))
  (bind _player (`self.Player`))
  (`/Engine/EditorBlueprintResources/StandardMacros.IsValid` _player
    (:`Is Valid`
      (bind (_valid_ _location) (message `/Game/BP/iface/InteractableInterface.GetGunLocation` _player))
      (if _valid_
        (`ParticleSystemComponent.SetBeamSourcePoint` (`self.ParticleSystem`) 0 _location 0)))))

(event `self.Cylinder1.OnComponentBeginOverlap`
  (params (OverlappedComponent :type "PrimitiveComponent Object Reference") (OtherActor :type "Actor Object Reference") (OtherComp :type "PrimitiveComponent Object Reference") (OtherBodyIndex :type Integer) (bFromSweep :type Boolean) (SweepResult :type "HitResult Structure (by ref)"))
  (`/Engine/EditorBlueprintResources/StandardMacros.IsValid` OtherActor
    (:`Is Valid`
      (if (`ActorComponent.ComponentHasTag` OtherComp "ImABoss")
        (switch `int` (`KismetArrayLibrary.Array_Find` (`self.ObjTypeInd`) (`KismetSystemLibrary.GetClassDisplayName` (`GameplayStatics.GetObjectClass` OtherActor)))
          (:`0`
            (bind _asbp_virus_boss_1 (cast `/Game/Maps/Heart/BPs/BP_Virus_Boss1` OtherActor))
            (`/Game/Maps/Heart/BPs/BP_Virus_Boss1.wrongWeapon` _asbp_virus_boss_1))
          (:`1`
            (bind _asbp_virus_boss_2 (cast `/Game/Maps/Heart/BPs/BP_VirusBoss2` OtherActor))
            (`/Game/Maps/Heart/BPs/BP_VirusBoss2.wrongWeapon` _asbp_virus_boss_2))
          (:`2`
            (bind _asbp_virus_boss_3 (cast `/Game/Maps/Heart/BPs/BP_VirusBoss3` OtherActor))
            (`/Game/Maps/Heart/BPs/BP_VirusBoss3.wrongWeapon` _asbp_virus_boss_3)))))))

(fn `UserConstructionScript`
  (bind _trace_distance (`self.Trace Distance`))
  (bind _cylinder (`self.Cylinder`))
  (`SceneComponent.SetRelativeScale3D` _cylinder (`KismetMathLibrary.MakeVector` 0.2 0.2 (/ _trace_distance 100.0)))
  (`SceneComponent.K2_SetRelativeLocation` _cylinder (`KismetMathLibrary.MakeVector` (/ _trace_distance 2.0)) false false)
  (`self.SetLifeSpan` (`self.LifeTime`)))