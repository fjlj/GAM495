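; BP_BombShot is a bomb projectile that explodes on impact.
; A looping timer sphere-traces from its previous to current location, ignoring the player character, to catch hits between updates.
; A hit spawns sparks and a BP_Explosion actor, then destroys the shot.
; Its cylinder overlap detects components tagged as bosses and calls WrongWeapon on the matching virus boss, resolved by class-name lookup.
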(event `self.Cylinder1.OnComponentBeginOverlap`
  (params (OverlappedComponent :type "PrimitiveComponent Object Reference") (OtherActor :type "Actor Object Reference") (OtherComp :type "PrimitiveComponent Object Reference") (OtherBodyIndex :type Integer) (bFromSweep :type Boolean) (SweepResult :type "HitResult Structure (by ref)"))
  (`/Engine/EditorBlueprintResources/StandardMacros.IsValid` OtherActor
    (:`Is Valid`
      (if (`ActorComponent.ComponentHasTag` OtherComp "ImABoss")
        (switch `int` (`KismetArrayLibrary.Array_Find` (`self.ObjTypeInd`) (`KismetSystemLibrary.GetClassDisplayName` (`GameplayStatics.GetObjectClass` OtherActor)))
          (:`0`
            (bind _asbp_virus_boss_1 (cast `/Game/Maps/Heart/BPs/BP_Virus_Boss1` OtherActor))
            (`/Game/Maps/Heart/BPs/BP_Virus_Boss1.wrongWeapon` _asbp_virus_boss_1))
          (:`1`
            (bind _asbp_virus_boss_2 (cast `/Game/Maps/Heart/BPs/BP_VirusBoss2` OtherActor))
            (`/Game/Maps/Heart/BPs/BP_VirusBoss2.wrongWeapon` _asbp_virus_boss_2))
          (:`2`
            (bind _asbp_virus_boss_3 (cast `/Game/Maps/Heart/BPs/BP_VirusBoss3` OtherActor))
            (`/Game/Maps/Heart/BPs/BP_VirusBoss3.wrongWeapon` _asbp_virus_boss_3)))))))

(event `self.ReceiveBeginPlay`
  (set `self.PreviousLocation` (`self.K2_GetActorLocation`))
  (bind _returnvalue (`KismetSystemLibrary.K2_SetTimerDelegate` (delegate `Tick`) (`self.TickFrequency`) true))
  (set `self.TickTimer` _returnvalue)
  (`self.Tick`))

(event `Tick`
  (bind (_outhit _returnvalue) (`KismetSystemLibrary.SphereTraceSingleForObjects` (`self.PreviousLocation`) (`self.K2_GetActorLocation`) (`self.TraceRadius`) (`|MakeArray` "ObjectTypeQuery1" "ObjectTypeQuery2" "ObjectTypeQuery3" :!type "EObjectTypeQuery Enum") false (`|MakeArray` (`GameplayStatics.GetPlayerCharacter` 0) :!type "Actor Object Reference") (select `bool` (`self.Debug?`) :`true` "ForDuration" :!type "EDrawDebugTrace Enum")))
  (if _returnvalue
    (`self.SpawnParticle&Damage` (`.ImpactPoint` (`GameplayStatics.BreakHitResult` _outhit)))
    (`KismetSystemLibrary.K2_ClearAndInvalidateTimerHandle` (`self.TickTimer`))
    (`self.K2_DestroyActor`)
    (else
      (set `self.PreviousLocation` (`self.K2_GetActorLocation`)))))

(event `SpawnParticle&Damage`
  (params (Location :type "Vector Structure"))
  (`GameplayStatics.SpawnEmitterAtLocation` "/Game/GFX/Particles/P_SparksFlair.P_SparksFlair" Location (struct) (0.5 0.5 0.5))
  (`|SpawnActorFromClass` "/Game/BP/Projectiles/BP_Explosion.BP_Explosion_C" (`KismetMathLibrary.MakeTransform` Location) "Undefined" "OverrideRootScale" null null))

(fn `UserConstructionScript`)